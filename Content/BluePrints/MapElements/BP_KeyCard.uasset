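; BP_KeyCard is a key card map element that the player can pick up.
; Character overlap turns the card grey until collected; ending overlap restores blue and clears the collected flag.
; Interact on the Trigger component snaps it to the supplied target point, marks it collected, and disables physics and sets Pawn collision to Ignore.
; It then registers KeyCard as the picked-up item on the player's NewNoNameCharacter.
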(event `self.KeyCard.OnComponentBeginOverlap`
  (params (OverlappedComponent :type "PrimitiveComponent Object Reference") (OtherActor :type "Actor Object Reference") (OtherComp :type "PrimitiveComponent Object Reference") (OtherBodyIndex :type Integer) (bFromSweep :type Boolean) (SweepResult :type "HitResult Structure (by ref)"))
  ;[1 1 1] Change Color when Near
  (if (not (`self.bBeenCollected`))
    (cast `Character` OtherActor)
    (`PrimitiveComponent.SetMaterial` (`self.KeyCard`) 0 "/Game/Materials/M_Grey.M_Grey")))

(event `self.KeyCard.OnComponentEndOverlap`
  (params (OverlappedComponent :type "PrimitiveComponent Object Reference") (OtherActor :type "Actor Object Reference") (OtherComp :type "PrimitiveComponent Object Reference") (OtherBodyIndex :type Integer))
  ;[1 1 1] Change Color when Near
  (cast `Character` OtherActor)
  (`PrimitiveComponent.SetMaterial` (`self.KeyCard`) 0 "/Game/Materials/M_Blue.M_Blue")
  (set `self.bBeenCollected` false))

(fn `Interact`
  (params (TargetPoint :type "SceneComponent Object Reference") (Component :type "PrimitiveComponent Object Reference"))
  (returns (Val :type Boolean))
  (if (== Component (`self.Trigger`))
    (`self.K2_AttachToComponent` TargetPoint "None" "SnapToTarget" "SnapToTarget" "KeepRelative")
    (set `self.bBeenCollected` true)
    (`PrimitiveComponent.SetMaterial` (`self.KeyCard`) 0 "/Game/Materials/M_Blue.M_Blue")
    (`PrimitiveComponent.SetCollisionResponseToChannel` (`self.KeyCard`) "ECC_Pawn" "ECR_Ignore")
    (`PrimitiveComponent.SetSimulatePhysics` (`self.KeyCard`) false)
    (bind _asnew_no_name_character (cast `/Game/BluePrints/Character/NewNoNameCharacter` (`GameplayStatics.GetPlayerCharacter` 0)))
    (set `/Game/BluePrints/Character/NewNoNameCharacter.ActorthatwasPickedUp` (`self.KeyCard`) _asnew_no_name_character)
    (return false)))

(fn `UserConstructionScript`)