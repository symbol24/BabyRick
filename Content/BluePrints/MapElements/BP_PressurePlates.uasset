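; Pressure plate that raises or lowers linked platforms when one designated actor, ObjectToOpen, enters or leaves its trigger.
; After a short delay, begin overlap calls MovePlatform on each PlatformsToMove entry and sends InteractMessage to ObjectToOpen with the Scene target point.
; End overlap clears ActorOverlapingWith and calls MoveDowm on each platform.
; Both loop bodies end in a Delay, which does not pause iteration.
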(event `self.Trigger.OnComponentBeginOverlap`
  (params (OverlappedComponent :type "PrimitiveComponent Object Reference") (OtherActor :type "Actor Object Reference") (OtherComp :type "PrimitiveComponent Object Reference") (OtherBodyIndex :type Integer) (bFromSweep :type Boolean) (SweepResult :type "HitResult Structure (by ref)"))
  (bind _objecttoopen_ (`self.ObjectToOpen `))
  (`KismetSystemLibrary.Delay` 0.2)
  (if (== OtherActor _objecttoopen_)
    (for _array_element (`self.PlatformsToMove`)
      (`/Game/BluePrints/MapElements/BP_MovePlatform.MovePlatform` _array_element)
      (message `/Game/BluePrints/Interfaces/BP_InteractableInterface.Interact` _objecttoopen_ (`self.Scene`) null)
      (`KismetSystemLibrary.Delay` 1.0))))

(event `self.Trigger.OnComponentEndOverlap`
  (params (OverlappedComponent :type "PrimitiveComponent Object Reference") (OtherActor :type "Actor Object Reference") (OtherComp :type "PrimitiveComponent Object Reference") (OtherBodyIndex :type Integer))
  (`KismetSystemLibrary.Delay` 0.2)
  (if (== (`self.ObjectToOpen `) OtherActor)
    (set `self.ActorOverlapingWith` null)
    (for _array_element (`self.PlatformsToMove`)
      (`/Game/BluePrints/MapElements/BP_MovePlatform.MoveDowm` _array_element)
      (`KismetSystemLibrary.Delay` 1.0))))

(fn `UserConstructionScript`)