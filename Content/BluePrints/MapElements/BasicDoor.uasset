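; BasicDoor is a map element door that swings open and shut on its yaw through OpenDoor and CloseDoor events.
; An IsOpen flag guards both events against repeats.
; GetRelativeRotAndLoc offsets the door mesh's current yaw, keeping its location, to feed an eased MoveComponentTo.
; Targets are relative to the current rotation rather than stored angles, and CloseDoor's move node shows no Component input.
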(event `self.ReceiveBeginPlay`)

(event `OpenDoor`
  (if (not (`self.IsOpen`))
    (set `self.IsOpen` true)
    (bind (_sm_door _relativelocation _returnvalue) (`self.GetRelativeRotAndLoc` 80.0))
    (`KismetSystemLibrary.MoveComponentTo` _sm_door _relativelocation _returnvalue true true 0.8)))

(event `CloseDoor`
  (if (`self.IsOpen`)
    (set `self.IsOpen` false)
    (bind (_sm_door _relativelocation _returnvalue) (`self.GetRelativeRotAndLoc` -80.0))
    (`KismetSystemLibrary.MoveComponentTo` null _relativelocation _returnvalue true true 0.8)))

(fn `GetRelativeRotAndLoc`
  (params (AmountToTurn :type "Float (double-precision)"))
  (returns (SM_Door :type "StaticMeshComponent Object Reference") (RelativeLocation :type "Vector Structure") (ReturnValue :type "Rotator Structure"))
  (bind _sm_door (`self.SM_Door`))
  (bind (_relativerotation_roll _relativerotation_pitch _relativerotation_yaw) (`KismetMathLibrary.BreakRotator` (`SceneComponent.RelativeRotation` _sm_door)))
  (return _sm_door (`SceneComponent.RelativeLocation` _sm_door) (`KismetMathLibrary.MakeRotator` _relativerotation_roll _relativerotation_pitch (- _relativerotation_yaw AmountToTurn))))

(fn `UserConstructionScript`)