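; BP_TerminalKeyCard is an interactable map terminal that activates only when its linked key card has been collected.
; Interact casts the owner of the referenced key card to BP_KeyCard and checks its BeenCollected flag.
; If collected, the terminal stops colliding with the Pawn channel and calls ActivateTerminal, which currently only prints a debug message.
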(event `ActivateTerminal`
  (`KismetSystemLibrary.PrintString` "Activated"))

(fn `Interact`
  (params (TargetPoint :type "SceneComponent Object Reference") (Component :type "PrimitiveComponent Object Reference"))
  (returns (Val :type Boolean))
  (bind _asbp_key_card (cast `/Game/BluePrints/MapElements/BP_KeyCard` (`ActorComponent.GetOwner` (`/Game/BluePrints/MapElements/BP_KeyCard.KeyCard` (`self.KeyCard?`)))))
  (if (`/Game/BluePrints/MapElements/BP_KeyCard.bBeenCollected` _asbp_key_card)
    (`PrimitiveComponent.SetCollisionResponseToChannel` (`self.Terminal`) "ECC_Pawn" "ECR_Ignore")
    (`self.ActivateTerminal`)
    (return false)))

(fn `UserConstructionScript`)