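; RealBabyRick is a map element that the player picks up through its Interact function.
; Interact makes the baby body ignore Pawn collision, stops its physics simulation, and snaps the pickup to the supplied target point.
; It then records the body as the picked-up object on NewNoNameCharacter and sets IsHeld on the player's NeverGonnaGiveYouUp component.
; The event graph and construction script are empty.
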(fn `Interact`
  (params (TargetPoint :type "SceneComponent Object Reference") (Component :type "PrimitiveComponent Object Reference"))
  (returns (Val :type Boolean))
  (bind _returnvalue (`GameplayStatics.GetPlayerCharacter` 0))
  (`PrimitiveComponent.SetCollisionResponseToChannel` (`self.babybody`) "ECC_Pawn" "ECR_Ignore")
  (`PrimitiveComponent.SetSimulatePhysics` (`self.babybody`) false)
  (`self.K2_AttachToComponent` TargetPoint "None" "SnapToTarget" "SnapToTarget" "KeepRelative")
  (bind _asnew_no_name_character (cast `/Game/BluePrints/Character/NewNoNameCharacter` _returnvalue))
  (set `/Game/BluePrints/Character/NewNoNameCharacter.ActorthatwasPickedUp` (`self.babybody`) _asnew_no_name_character)
  (set `/Game/BluePrints/Character/NeverGonnaGiveYouUp.IsHeld` true (`self.GetComponentByClass` _returnvalue "/Game/BluePrints/Character/NeverGonnaGiveYouUp.NeverGonnaGiveYouUp_C"))
  (return false))

(fn `UserConstructionScript`)