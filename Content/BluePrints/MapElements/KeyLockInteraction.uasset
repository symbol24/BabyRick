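; KeyLockInteraction provides a KeyLockSystem function that reports a pressure plate's holding state and a button's lock state.
; It casts the owners of the two inputs' scene roots to BP_PressurePlates and BP_NewButton, then returns HoldingObject and IsLocked.
; A Sequence feeds both branches into one return, so a holding plate returns before the button cast runs.
; It changes neither actor, and the event graph is empty.
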(fn `KeyLockSystem`
  (params (PressurePlate :type "/Game/BluePrints/MapElements/BP_PressurePlates Object Reference") (ButtonToPress :type "/Game/BluePrints/MapElements/BP_NewButton Object Reference"))
  (returns (`HoldingObject?` :type Boolean) (`IsLocked?` :type Boolean))
  (`|ExecutionSequence`
    (:`then_0`
      (bind _asbp_pressure_plates (cast `/Game/BluePrints/MapElements/BP_PressurePlates` (`self.GetOwner` (`/Game/BluePrints/MapElements/BP_PressurePlates.DefaultSceneRoot` PressurePlate))))
      (bind _holdingobject (`/Game/BluePrints/MapElements/BP_PressurePlates.HoldingObject` _asbp_pressure_plates))
      (if _holdingobject
        (return _holdingobject (`/Game/BluePrints/MapElements/BP_NewButton.IsLocked?` (stale _asbp_new_button)))))
    (:`then_1`
      (bind _asbp_new_button (cast `/Game/BluePrints/MapElements/BP_NewButton` (`self.GetOwner` (`/Game/BluePrints/MapElements/BP_NewButton.DefaultSceneRoot` ButtonToPress))))
      (return _holdingobject (`/Game/BluePrints/MapElements/BP_NewButton.IsLocked?` _asbp_new_button)))))