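; BP_NewButton is an interactable button that moves a set of linked platforms, alternating direction on each press.
; Interact sets a WasHit guard and fires ActivateButton, which greys the button, plays a switch sound and uses a FlipFlop to call MovePlatform or MoveDowm on AllPlatformsToMove.
; Short delays restore the material, then re-arm the guard and DoOnce.
; The press-animation timeline and single-platform casts are disconnected.
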(event `self.ReceiveBeginPlay`
  (set `self.StartPos` (`SceneComponent.RelativeLocation` (`self.Button`)))
  (`PrimitiveComponent.SetMaterial` (`self.Button`) 0 (`self.Material`)))

(event `ActivateButton`
  ;[1 1 1] Comment
  (`/Engine/EditorBlueprintResources/StandardMacros.DoOnce` false :!label _label
    (:`Completed`
      (`PrimitiveComponent.SetMaterial` (`self.Button`) 0 "/Game/Materials/M_Grey.M_Grey")
      (`GameplayStatics.PlaySound2D` "/Game/SFX/switch-2.switch-2")
      (`|ExecutionSequence`
        (:`then_0`
          (`/Engine/EditorBlueprintResources/StandardMacros.FlipFlop`
            (:`A`
              (for _array_element (`self.AllPlatformsToMove`)
                (`/Game/BluePrints/MapElements/BP_MovePlatform.MovePlatform` _array_element)))
            (:`B`
              (for _array_element_2 (`self.AllPlatformsToMove`)
                (`/Game/BluePrints/MapElements/BP_MovePlatform.MoveDowm` _array_element_2))))
          (`KismetSystemLibrary.Delay` 1.0)
          (set `self.WasHit` false)
          (`self.Reset`))
        (:`then_1`
          (`KismetSystemLibrary.Delay` 0.5)
          (`PrimitiveComponent.SetMaterial` (`self.Button`) 0 (`self.Material`)))))))

(event `Reset`
  (goto _label :!via `Reset`))

(fn `Interact`
  (params (TargetPoint :type "SceneComponent Object Reference") (Component :type "PrimitiveComponent Object Reference"))
  (returns (Val :type Boolean))
  (if (not (`self.WasHit`))
    (set `self.WasHit` true)
    (`self.ActivateButton`)
    (return false)))

(fn `UserConstructionScript`)