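; BP_MovePlatform is a map element that slides its Platform component along a configurable XYZ offset.
; MovePlatform adds the axis offsets to the current relative location, while MoveDowm targets the offsets minus that location, which is a true return only from specific positions.
; Both events ease in and out over TimeToMove, keep rotation unchanged, and use an IsMoving flag to ignore calls mid-move.
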(event `MovePlatform`
  (bind _platform (`self.Platform`))
  (bind (_relativelocation_x _relativelocation_y _relativelocation_z) (`KismetMathLibrary.BreakVector` (`SceneComponent.RelativeLocation` _platform)))
  (if (not (`self.is moving`))
    (set `self.is moving` true)
    (`KismetSystemLibrary.MoveComponentTo` _platform (`KismetMathLibrary.MakeVector` (+ _relativelocation_x (`self.XAxis`)) (+ _relativelocation_y (`self.YAxis`)) (+ _relativelocation_z (`self.ZAxis`))) (`SceneComponent.RelativeRotation` _platform) true true (`self.TimeToMove`))
    (set `self.is moving` false)))

(event `MoveDowm`
  (bind _platform (`self.Platform`))
  (bind (_relativelocation_x _relativelocation_y _relativelocation_z) (`KismetMathLibrary.BreakVector` (`SceneComponent.RelativeLocation` _platform)))
  (if (not (`self.is moving`))
    (set `self.is moving` true)
    (`KismetSystemLibrary.MoveComponentTo` _platform (`KismetMathLibrary.MakeVector` (- (`self.XAxis`) _relativelocation_x) (- (`self.YAxis`) _relativelocation_y) (- (`self.ZAxis`) _relativelocation_z)) (`SceneComponent.RelativeRotation` _platform) true true (`self.TimeToMove`))
    (set `self.is moving` false)))

(fn `UserConstructionScript`)