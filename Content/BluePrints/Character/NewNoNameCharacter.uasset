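; NewNoNameCharacter is a first-person character Blueprint that lets the player interact with nearby objects.
; Trigger overlaps track the last actor implementing BP_InteractableInterface and clear it, along with CanInteract, on exit.
; When interaction is allowed, the Interact input runs a short debug-drawn camera line trace on Visibility.
; It sends InteractMessage to the stored actor with the Hand and the first hit component, without checking the trace hit anything.
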(event `self.Trigger.OnComponentBeginOverlap`
  (params (OverlappedComponent :type "PrimitiveComponent Object Reference") (OtherActor :type "Actor Object Reference") (OtherComp :type "PrimitiveComponent Object Reference") (OtherBodyIndex :type Integer) (bFromSweep :type Boolean) (SweepResult :type "HitResult Structure (by ref)"))
  ;[1 1 1] ColidingWith Objects to Interact
  (if (`KismetSystemLibrary.DoesImplementInterface` OtherActor "/Game/BluePrints/Interfaces/BP_InteractableInterface.BP_InteractableInterface_C")
    (set `self.bCanInteract` true)
    (set `self.InteractableActor` OtherActor)))

(event `self.Trigger.OnComponentEndOverlap`
  (params (OverlappedComponent :type "PrimitiveComponent Object Reference") (OtherActor :type "Actor Object Reference") (OtherComp :type "PrimitiveComponent Object Reference") (OtherBodyIndex :type Integer))
  ;[1 1 1] ColidingWith Objects to Interact
  (if (`KismetSystemLibrary.DoesImplementInterface` OtherActor "/Game/BluePrints/Interfaces/BP_InteractableInterface.BP_InteractableInterface_C")
    (set `self.bCanInteract` false)
    (set `self.InteractableActor` null)))

(event `InputAction|Interact`
  (params (Key :type "Key Structure"))
  (bind _firstpersoncamera (`self.FirstPersonCamera`))
  (bind _returnvalue (`SceneComponent.K2_GetComponentLocation` _firstpersoncamera))
  ;[1 1 1] Interact With Objects
  (:`Pressed`
    (if (`self.bCanInteract`)
      (bind _outhits (`KismetSystemLibrary.LineTraceMulti` :`Start` _returnvalue :`End` (+ _returnvalue (* (`SceneComponent.GetForwardVector` _firstpersoncamera) 200.0)) :`TraceChannel` "TraceTypeQuery1" :`DrawDebugType` "ForDuration"))
      (bind (_output_bblockinghit _output_binitialoverlap _output_time _output_distance _output_location _output_impactpoint _output_normal _output_impactnormal _output_physmat _output_hitactor _output_hitcomponent) (`GameplayStatics.BreakHitResult` (`|GetArrayItem` _outhits)))
      (message `/Game/BluePrints/Interfaces/BP_InteractableInterface.Interact` (`self.InteractableActor`) (`self.Hand`) _output_hitcomponent))))

(fn `UserConstructionScript`
  (`parent.UserConstructionScript`))