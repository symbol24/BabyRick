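; Character component that tracks player anxiety around a RealBabyRick actor, found in the level shortly after BeginPlay.
; Each tick Anxiety falls while IsHeld is true and rises otherwise, clamped between zero and MaxAnxiety.
; The value maps to four states by thirds and maximum, feeding the owning NewNoNameCharacter's UI and ToggleDepressed call.
; At maximum anxiety, it tells Rick to TeleportAway, gated by a five-second cooldown.
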(event `self.ReceiveBeginPlay`
  (`KismetSystemLibrary.Delay` 0.01)
  (bind _outactors (`GameplayStatics.GetAllActorsOfClass` "/Game/BluePrints/MapElements/RealBabyRick.RealBabyRick_C"))
  (if (> (`KismetArrayLibrary.Array_Length` _outactors) 0)
    (set `self.Rick` (`|GetArrayItem` _outactors))
    (else
      (`KismetSystemLibrary.PrintString` "No Baby Rick Found!!! OMG!"))))

(event `self.ReceiveTick`
  (params (DeltaSeconds :type "Float (single-precision)"))
  (`self.ChangeAnxiety`)
  (`self.SetAnxiousAndDepressed`)
  (if (`|EnumEquality` (`self.AnxietyState`) "NewEnumerator3")
    (`self.BabyTeleport`)))

(event `BabyTeleport`
  (if (`self.CanTeleport`)
    (set `self.CanTeleport` false)
    (`/Game/BluePrints/MapElements/RealBabyRick.TeleportAway` (`self.Rick`))
    (`KismetSystemLibrary.Delay` 5.0)
    (set `self.CanTeleport` true)))

(fn `ChangeAnxiety`
  (`KismetSystemLibrary.PrintString` (`KismetStringLibrary.Conv_BoolToString` (`self.IsHeld`)))
  (if (`self.IsHeld`)
    (set `self.Anxiety` (`KismetMathLibrary.FClamp` (- (`self.Anxiety`) 0.001) 0.0 (`self.MaxAnxiety`)))
    (else
      (set `self.Anxiety` (`KismetMathLibrary.FClamp` (+ (`self.Anxiety`) 0.001) 0.0 (`self.MaxAnxiety`))))))

(fn `SetAnxiousAndDepressed`
  (locals (character :type "/Game/BluePrints/Character/NewNoNameCharacter Object Reference"))
  (bind _asnew_no_name_character (cast `/Game/BluePrints/Character/NewNoNameCharacter` (`self.GetOwner`)))
  (set `local.character` _asnew_no_name_character)
  (`|ExecutionSequence`
    (:`then_0`
      (if (== (`self.Anxiety`) (`self.MaxAnxiety`))
        (set `self.AnxietyState` "NewEnumerator3")
        (elif (>= (`self.Anxiety`) (+ (/ (`self.MaxAnxiety`) 3.0) (/ (`self.MaxAnxiety`) 3.0)))
          (set `self.AnxietyState` "NewEnumerator2")
          (elif (>= (`self.Anxiety`) (/ (`self.MaxAnxiety`) 3.0))
            (set `self.AnxietyState` "NewEnumerator1")
            (else
              (set `self.AnxietyState` "NewEnumerator0"))))))
    (:`then_1`
      (`/Game/BluePrints/Widgets/PlayerUI.UpdateAnxiety` (`/Game/BluePrints/Character/NewNoNameCharacter.PlayerUI` (`local.character`)) (/ (`self.Anxiety`) (`self.MaxAnxiety`)) (`self.AnxietyState`)))
    (:`then_2`
      (bind _asnew_no_name_character_2 (cast `/Game/BluePrints/Character/NewNoNameCharacter` (`self.GetOwner`)))
      (`/Game/BluePrints/Character/NewNoNameCharacter.ToggleDepressed` _asnew_no_name_character_2))))