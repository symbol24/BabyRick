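; BabyRickGameMode is a game mode that handles background music and basic game flow for the game.
; Events pause the game on game over, open RoomsMap, or reload the current level by name.
; BeginPlay calls the normal music event, which adds a scene component to the player character when no sound exists.
; The IsPlayingAnxious flag gates switching between normal and anxious tracks, stopping the current sound and spawning the next attached to that component.
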(event `self.ReceiveBeginPlay`
  (`self.PlayNormalMusic`))

(event `GameOver`
  (`GameplayStatics.SetGamePaused` true))

(event `LoadLevel`
  (`GameplayStatics.OpenLevel` "RoomsMap"))

(event `RestartLevel`
  (bind _returnvalue (`GameplayStatics.GetCurrentLevelName` true))
  (`GameplayStatics.OpenLevel` (`KismetStringLibrary.Conv_StringToName` _returnvalue)))

(event `PlayNormalMusic`
  (bind _soundplaying (`self.SoundPlaying`))
  (if (`self.IsPlayingAnxious`)
    (set `self.IsPlayingAnxious` false)
    (`/Engine/EditorBlueprintResources/StandardMacros.IsValid` _soundplaying
      (:`Is Valid`
        (if (`AudioComponent.IsPlaying` _soundplaying)
          (`AudioComponent.Stop` (`self.SoundPlaying`))))
      (:`Is Not Valid`
        (bind _returnvalue (`AddComponent|NODE_AddSceneComponent-0` :`self` (`GameplayStatics.GetPlayerCharacter` 0)))
        (set `self.SceneComp` _returnvalue)))
    (bind _returnvalue_2 (`GameplayStatics.SpawnSoundAttached` (`self.BackgroundMusic`) (`self.SceneComp`)))
    (set `self.SoundPlaying` _returnvalue_2)))

(event `PlayAnxiousMusic`
  (if (not (`self.IsPlayingAnxious`))
    (set `self.IsPlayingAnxious` true)
    (if (`AudioComponent.IsPlaying` (`self.SoundPlaying`))
      (`AudioComponent.Stop` (`self.SoundPlaying`)))
    (bind _returnvalue (`GameplayStatics.SpawnSoundAttached` (`self.AnxiousSoundCue`) (`self.SceneComp`)))
    (set `self.SoundPlaying` _returnvalue)))

(fn `UserConstructionScript`)